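; BP_Tile is a clickable grid tile that takes on the biome currently selected on the player's BP_TopDownCharacter.
; Clicking its Plane copies that biome, prints it and calls UpdateBiomeVisuals, which destroys previously spawned actors and spawns new ones.
; Grassland, Forest and Mountain scatter random picks around the tile and set a grass material, with Mountain reusing ForestActors.
; Water and Town spawn every class in their arrays at the tile's location.
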(event OnClicked(Plane)
  (params (TouchedComponent :type Primitive%20Component%20Object%20Reference) (ButtonPressed :type Key%20Structure :default "None"))
  (bind _asbp_top_down_character (Utilities|Casting|CastToBP_TopDownCharacter (Game|GetPlayerCharacter 0)))
  (bind _output_get (Variables|Default|SetTileBiome (Variables|/Game/TopDown/Blueprints/BP_TopDownCharacter.BP_TopDownCharacter_C|GetSelectedBiome _asbp_top_down_character)))
  (Development|PrintString (Utilities|String|EnumtoString _output_get))
  (CallFunction|UpdateBiomeVisuals))

(event EventBeginPlay)

(event Collision|EventActorBeginOverlap
  (params (OtherActor :type Actor%20Object%20Reference)))

(event EventTick
  (params (DeltaSeconds :type Float%20%28single-precision%29)))

(fn ConstructionScript)

(fn UpdateBiomeVisuals
  (bind _returnvalue (Math|Random|RandomFloatinRange -75.0 75.0))
  (bind _returnvalue_2 (Math|Random|RandomFloatinRange -5e+01 5e+01))
  (bind _returnvalue_3 (Math|Random|RandomFloatinRange -5e+01 5e+01))
  (bind _spawnedactors (Variables|Default|GetSpawnedActors))
  (for _array_element _spawnedactors
    (Actor|DestroyActor _array_element))
  (Utilities|Array|Clear _spawnedactors)
  (switch Utilities|FlowControl|Switch|SwitchonE_BiomeType (Variables|Default|GetTileBiome)
    (:NewEnumerator0
      ;[0.15 0.15 0.15 0.5] Grassland-> randomly spawning
      (for _index (range 1 (Variables|Default|GetSpawnCount))
        (Game|SpawnActorfromClass (Utilities|Array|Get(acopy) (Variables|Default|GetGrasslandActors) (Math|Random|RandomIntegerinRange 0 (- (Utilities|Array|Length (Variables|Default|GetGrasslandActors)) 1))) (Math|Transform|MakeTransform (+ (Transformation|GetActorLocation) (Math|Vector|MakeVector _returnvalue _returnvalue 0.0)) (Math|Conversions|RotationFromXVector (Math|Vector|MakeVector (Math|Random|RandomFloat) 0.0 0.0))) "AlwaysSpawn" "MultiplyWithRoot" 0 0)
        (Utilities|Array|Add (Variables|Default|GetSpawnedActors) 0)
        (Rendering|Material|SetMaterial (Variables|Default|GetPlane) 0 "/Game/Assets/CozyNature/Textures/Terrain/Grass.Grass")))
    (:NewEnumerator1
      ;[0.15 0.15 0.15 0.5] Water section
      (for _array_element_2 (Variables|Default|GetWaterActors)
        (bind _returnvalue_4 (Game|SpawnActorfromClass _array_element_2 (Math|Transform|MakeTransform (Transformation|GetActorLocation)) "AlwaysSpawn" "MultiplyWithRoot" 0 0))
        (Utilities|Array|Add (Variables|Default|GetSpawnedActors) _returnvalue_4)))
    (:NewEnumerator2
      ;[0.15 0.15 0.15 0.5] Forest
      (for _index_2 (range 1 (Variables|Default|GetSpawnCount))
        (Game|SpawnActorfromClass (Utilities|Array|Get(acopy) (Variables|Default|GetForestActors) (Math|Random|RandomIntegerinRange 0 (- (Utilities|Array|Length (Variables|Default|GetForestActors)) 1))) (Math|Transform|MakeTransform (+ (Transformation|GetActorLocation) (Math|Vector|MakeVector _returnvalue_3 _returnvalue_3 0.0)) (Math|Conversions|RotationFromXVector (Math|Vector|MakeVector (Math|Random|RandomFloat) 0.0 0.0))) "AlwaysSpawn" "MultiplyWithRoot" 0 0)
        (Utilities|Array|Add (Variables|Default|GetSpawnedActors) 0)
        (Rendering|Material|SetMaterial (Variables|Default|GetPlane) 0 "/Game/Assets/CozyNature/Textures/Terrain/Grass.Grass")))
    (:NewEnumerator3
      ;[0.15 0.15 0.15 0.5] Town
      (for _array_element_3 (Variables|Default|GetTownActors)
        (bind _returnvalue_5 (Game|SpawnActorfromClass _array_element_3 (Math|Transform|MakeTransform (Transformation|GetActorLocation)) "AlwaysSpawn" "MultiplyWithRoot" 0 0))
        (Utilities|Array|Add (Variables|Default|GetSpawnedActors) _returnvalue_5)))
    (:NewEnumerator4
      ;[0.15 0.15 0.15 0.5] Mountain
      (for _index_3 (range 1 (Variables|Default|GetSpawnCount))
        (Game|SpawnActorfromClass (Utilities|Array|Get(acopy) (Variables|Default|GetForestActors) (Math|Random|RandomIntegerinRange 0 (- (Utilities|Array|Length (Variables|Default|GetForestActors)) 1))) (Math|Transform|MakeTransform (+ (Transformation|GetActorLocation) (Math|Vector|MakeVector _returnvalue_2 _returnvalue_2 0.0)) (Math|Conversions|RotationFromXVector (Math|Vector|MakeVector (Math|Random|RandomFloat) 0.0 0.0))) "AlwaysSpawn" "MultiplyWithRoot" 0 0)
        (Utilities|Array|Add (Variables|Default|GetSpawnedActors) 0)
        (Rendering|Material|SetMaterial (Variables|Default|GetPlane) 0 "/Game/Assets/CozyNature/Textures/Terrain/Grass.Grass")))))